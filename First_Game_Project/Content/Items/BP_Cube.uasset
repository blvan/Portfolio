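; BP_Cube is an interactable item that changes to a random color when interacted with.
; StartInterract sets the PaperFlipbook's sprite color to random RGB values at full alpha.
; A DoOnce, reset after a short Delay, acts as a cooldown against rapid repeat triggers.
; The default event stubs are disabled, and the construction script only calls its parent.
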(event EventBeginPlay
  (|CallParentFunction) ; This node is disabled and will not be called.\nDrag off pins to build functionality.
)

(event Collision|EventActorBeginOverlap
  (params (OtherActor :type Actor%20Object%20Reference))
  (|CallParentFunction OtherActor) ; This node is disabled and will not be called.\nDrag off pins to build functionality.
)

(event EventTick
  (params (DeltaSeconds :type Float%20%28single-precision%29))
  (|CallParentFunction DeltaSeconds) ; This node is disabled and will not be called.\nDrag off pins to build functionality.
)

(event EventStartInterract
  (Utilities|FlowControl|DoOnce false :!label _label
    (:Completed
      (Sprite|SetSpriteColor (Variables|Default|GetPaperFlipbook) (Utilities|Struct|MakeLinearColor (Math|Random|RandomFloat) (Math|Random|RandomFloat) (Math|Random|RandomFloat) 1.0))
      (Utilities|FlowControl|Delay 0.2)
      (goto _label Reset))))

(fn ConstructionScript
  (|CallParentFunction))