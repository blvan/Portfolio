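; BP_Interractable is an interactable actor that shows a widget and accepts interaction while the player character is inside its Box.
; Box overlap events toggle the widget and an interactable flag for the player character cached on BeginPlay.
; Tick polls that flag and the player's InterractPressed, using a DoOnce that resets when either is false to fire StartInterract once per press.
; StartInterract is an empty event here, leaving the response undefined.
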(event OnComponentBeginOverlap(Box)
  (params (OverlappedComponent :type Primitive%20Component%20Object%20Reference) (OtherActor :type Actor%20Object%20Reference) (OtherComp :type Primitive%20Component%20Object%20Reference) (OtherBodyIndex :type Integer) (bFromSweep :type Boolean) (SweepResult :type Hit%20Result%20Structure%20%28by%20ref%29))
  (if (== OtherActor (Variables|Default|GetPlayerCharacterRef))
    (Development|SetHiddeninGame (Variables|Default|GetWidget) false false)
    (Variables|Default|SetIsInterractable true)))

(event OnComponentEndOverlap(Box)
  (params (OverlappedComponent :type Primitive%20Component%20Object%20Reference) (OtherActor :type Actor%20Object%20Reference) (OtherComp :type Primitive%20Component%20Object%20Reference) (OtherBodyIndex :type Integer))
  (if (== (Variables|Default|GetPlayerCharacterRef) OtherActor)
    (Development|SetHiddeninGame (Variables|Default|GetWidget) true false)
    (Variables|Default|SetIsInterractable false)))

(event Custom|StartInterract)

(event EventBeginPlay
  (bind _asbp_player_character (Utilities|Casting|CastToBP_PlayerCharacter (Game|GetPlayerCharacter 0)))
  (Variables|Default|SetPlayerCharacterRef _asbp_player_character))

(event Collision|EventActorBeginOverlap
  (params (OtherActor :type Actor%20Object%20Reference)))

(event EventTick
  (params (DeltaSeconds :type Float%20%28single-precision%29))
  (if (and (Variables|Default|GetIsInterractable) (Variables|/Game/Characters/PlayerCharacter/BP_PlayerCharacter.BP_PlayerCharacter_C|GetInterractPressed (Variables|Default|GetPlayerCharacterRef)))
    (Utilities|FlowControl|DoOnce false :!label _label
      (:Completed
        (CallFunction|StartInterract)))
    (else
      (goto _label Reset))))

(fn ConstructionScript)