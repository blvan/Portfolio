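; Laser door item that toggles between open and closed when interacted with.
; StartInterract flips IsOpen, then switches collision between none and query-and-physics and swaps the Paper2D flipbook to match the new state.
; A DoOnce reset after a short delay debounces repeated interactions.
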(event EventBeginPlay
  (|CallParentFunction))

(event Collision|EventActorBeginOverlap
  (params (OtherActor :type Actor%20Object%20Reference))
  (|CallParentFunction OtherActor) ; This node is disabled and will not be called.\nDrag off pins to build functionality.
)

(event EventTick
  (params (DeltaSeconds :type Float%20%28single-precision%29))
  (|CallParentFunction DeltaSeconds) ; This node is disabled and will not be called.\nDrag off pins to build functionality.
)

(event EventStartInterract
  (Utilities|FlowControl|DoOnce false :!label _label
    (:Completed
      (bind _output_get (Variables|Default|SetIsOpen (not (Variables|Default|GetIsOpen))))
      (Collision|SetCollisionEnabled (Variables|Default|GetCollision) (select _output_get "NoCollision" "QueryAndPhysics"))
      (Sprite|SetFlipbook (Variables|Default|GetPaperFlipbook) (select _output_get (Variables|Default|GetFB_Opened) (Variables|Default|GetFB_Closed)))
      (Utilities|FlowControl|Delay 0.2)
      (goto _label Reset))))

(fn ConstructionScript
  (|CallParentFunction))