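; BP_Stormhead is an enemy character with a Paper2D flipbook sprite that defers BeginPlay, Tick and damage handling to its parent class.
; Tick adds signed movement input from MoveRight, but the zero direction vector produces no movement.
; AnyDamage prints the damage causer's name before calling the parent.
; Random direction, Run1 flipbook and sprite-flip logic is disconnected, and HandleRotation is empty.
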(event Game|Damage|EventAnyDamage
  (params (Damage :type Float%20%28single-precision%29) (DamageType :type Damage%20Type%20Object%20Reference) (InstigatedBy :type Controller%20Object%20Reference) (DamageCauser :type Actor%20Object%20Reference))
  (Development|PrintString (Utilities|GetDisplayName DamageCauser))
  (|CallParentFunction Damage DamageType InstigatedBy DamageCauser))

(event EventBeginPlay
  (|CallParentFunction))

(event EventTick
  (params (DeltaSeconds :type Float%20%28single-precision%29))
  ;[1 1 1] Rotarion
  ;;[1 0 0] Stopped
  (|CallParentFunction DeltaSeconds)
  (Pawn|Input|AddMovementInput "0, 0, 0" (select (Variables|Default|GetMoveRight) 1.0 -1.0) false))

(fn ConstructionScript)

(fn HandleRotation)