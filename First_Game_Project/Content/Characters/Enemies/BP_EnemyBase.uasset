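; BP_EnemyBase is a flipbook-animated enemy base character with clamped health and a widget health bar.
; Damage updates the bar and sets either IsDead or IsDamaged.
; Tick derives movement from velocity and selects idle, running or damaged flipbooks, using a delay to clear damage.
; Death animation and delayed destruction run only when IsDamaged is also set, which the lethal hit itself does not do.
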(event Custom|UpdateAnimation
  (if (Variables|Default|GetIsDamaged)
    (if (Variables|Default|GetIsDead)
      (CallFunction|Died)
      (Utilities|FlowControl|Delay (Class|PaperFlipbookComponent|GetFlipbookLength (Variables|Default|GetSprite)))
      (Actor|DestroyActor)
      (else
        (Sprite|SetFlipbook (Variables|Default|GetSprite) (select (Variables|Default|GetIsDamaged) (Variables|Default|GetFB_Damaged) (Variables|Default|GetFB_Idle)))
        (if (Variables|Default|GetIsDamaged)
          (Utilities|FlowControl|Delay (Class|PaperFlipbookComponent|GetFlipbookLength (Variables|Default|GetSprite)))
          (Variables|Default|SetIsDamaged false))))
    (elif (Variables|Default|Getismoving?)
      (Sprite|SetFlipbook (Variables|Default|GetSprite) (Variables|Default|GetFB_running))
      (else
        (Sprite|SetFlipbook (Variables|Default|GetSprite) (Variables|Default|GetFB_Idle))))))

(event Game|Damage|EventAnyDamage
  (params (Damage :type Float%20%28single-precision%29) (DamageType :type Damage%20Type%20Object%20Reference) (InstigatedBy :type Controller%20Object%20Reference) (DamageCauser :type Actor%20Object%20Reference))
  (CallFunction|UpdateHealth Damage))

(event EventTick
  (params (DeltaSeconds :type Float%20%28single-precision%29))
  (CallFunction|UpdateMovement)
  (CallFunction|UpdateAnimation))

(event EventBeginPlay
  (bind _aswbp_enemy_health (Utilities|Casting|CastToWBP_EnemyHealth (UserInterface|GetUserWidgetObject (Variables|Default|GetWidget))))
  (bind _output_get (Variables|Default|SetWBP_Enemy_HealthBarRef _aswbp_enemy_health))
  (Variables|/Game/Items/WBP_EnemyHealth.WBP_EnemyHealth_C|SetCharacterRef _output_get self)
  (Default|UpdateEnemyHealth (Variables|Default|GetWBP_Enemy_HealthBarRef)))

(fn ConstructionScript
  (Variables|Default|SetHealth (Variables|Default|GetDefaultHealth)))

(fn UpdateHealth
  (params (NewParam :type Float%20%28double-precision%29))
  (Variables|Default|SetHealth (Math|Float|Clamp(Float) (- (Variables|Default|GetHealth) NewParam) 0.0 (Variables|Default|GetDefaultHealth)))
  (Default|UpdateEnemyHealth (Variables|Default|GetWBP_Enemy_HealthBarRef))
  (if (and (<= (Variables|Default|GetHealth) 0.0) (not (Variables|Default|GetIsDead)))
    (Variables|Default|SetIsDead true)
    (else
      (Variables|Default|SetIsDamaged true))))

(fn Died
  (Sprite|SetFlipbook (Variables|Default|GetSprite) (Variables|Default|GetFB_Death)))

(fn UpdateMovement
  (Variables|Default|Setismoving? (> (Math|Vector|VectorLength (Pawn|Components|CharacterMovement|GetLastUpdateVelocity (Variables|Character|GetCharacterMovement))) 0.0)))